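; Game instance for an idle game that owns the save data and persists the last saved score.
; On Init it loads BP_SaveGame from the named slot, or creates a new one and prints a debug message if none exists.
; SaveGame writes the score to that slot, while LoadGame passes the stored score to BP_GameMode's GameLoaded.
; The LoadGame call in the event graph is disconnected, so Init does not trigger it.
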(event `self.ReceiveInit`
  (bind _returnvalue (`GameplayStatics.DoesSaveGameExist` (`self.SaveSlotName`)))
  (if _returnvalue
    (bind _returnvalue_2 (`GameplayStatics.LoadGameFromSlot` (`self.SaveSlotName`)))
    (bind _asbp_save_game (cast `/Game/Logic/BP_SaveGame` _returnvalue_2))
    (set `self.SaveGameData` _asbp_save_game)
    (else
      (bind _returnvalue_3 (`GameplayStatics.CreateSaveGameObject` "/Game/Logic/BP_SaveGame.BP_SaveGame_C"))
      (set `self.SaveGameData` _returnvalue_3)
      (`KismetSystemLibrary.PrintString` "Hello"))))

(fn `LoadGame`
  (bind _asbp_game_mode (cast `/Game/Logic/BP_GameMode` (`GameplayStatics.GetGameMode`)))
  (`/Game/Logic/BP_GameMode.GameLoaded` _asbp_game_mode (`/Game/Logic/BP_SaveGame.LastSavedScore` (`self.SaveGameData`))))

(fn `SaveGame`
  (params (LastSavedScore :type Integer64))
  (bind _savegamedata (`self.SaveGameData`))
  (set `/Game/Logic/BP_SaveGame.LastSavedScore` LastSavedScore _savegamedata)
  (`GameplayStatics.SaveGameToSlot` _savegamedata (`self.SaveSlotName`)))