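; Game mode for an idle clicker game that holds the player's score and drives the score display.
; On BeginPlay it creates the WBP_PlayerView widget and adds it to the viewport.
; Clicked raises the score by the click multiplier and GameLoaded sets it from a passed-in value, both pushing the result to the widget.
; SaveAndQuit saves through BP_IdleGameInstance, then quits the game.
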(event `self.ReceiveBeginPlay`
  (bind _returnvalue (`|CreateWidget` "/Game/UI/WBP_PlayerView.WBP_PlayerView_C"))
  (bind _output_get (set `self.UI` _returnvalue))
  (`UserWidget.AddToViewport` _output_get 0))

(event `SaveAndQuit`
  (bind _asbp_idle_game_instance (cast `/Game/Logic/BP_IdleGameInstance` (`GameplayStatics.GetGameInstance`)))
  (`/Game/Logic/BP_IdleGameInstance.SaveGame` _asbp_idle_game_instance)
  (`KismetSystemLibrary.QuitGame` null "Quit"))

(fn `Clicked`
  (bind _output_get (set `self.Score` (+ (`self.Score`) (* 1 (`self.ClickMultiplyer`)))))
  (set `/Game/UI/WBP_PlayerView.PlayersScore` _output_get (`self.UI`)))

(fn `GameLoaded`
  (params (Score :type Integer64))
  (bind _output_get (set `self.Score` Score))
  (set `/Game/UI/WBP_PlayerView.PlayersScore` _output_get (`self.UI`)))

(fn `UserConstructionScript`)